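; Player-pilotable spaceship pawn with physics-driven flight, a laser machine gun, health and crash damage.
; Enhanced Input applies acceleration-based forces and torques, with forward thrust smoothly scaling engine VFX and sound.
; Possession toggles physics, input and HUD, advances the quest and starts health regen; overlap shows a key prompt, and exiting requires a downward trace hit.
; Death triggers an explosion and delayed level restart.
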(event OnComponentHit(SpaceShipMesh)
  (params (HitComponent :type Primitive%20Component%20Object%20Reference) (OtherActor :type Actor%20Object%20Reference) (OtherComp :type Primitive%20Component%20Object%20Reference) (NormalImpulse :type Vector :default "0, 0, 0") (Hit :type Hit%20Result%20Structure%20%28by%20ref%29))
  (bind _returnvalue (Transformation|GetVelocity))
  (bind _returnvalue_2 (Math|Vector|VectorLength _returnvalue))
  ;[0.1042 0.1042 0.1042] HP System
  ;;[0.1042 0.1042 0.1042] Get Damage When Ship Crash Something
  (if (Variables|Default|Getis%20Get%20Damage%20For%20Crash)
    (if (> _returnvalue_2 1.5e+03)
      (CallFunction|UpdateHealth (* _returnvalue_2 -1.0 0.01))
      (Audio|PlaySound2D "/Game/-Yunus/Sounds/Explosion-Collison/MS_CrashShip.MS_CrashShip" 1.4 1.0 0.0 0 0 false)
      (Variables|Default|Setis%20Get%20Damage%20For%20Crash false)
      (Utilities|FlowControl|Delay 0.5)
      (Variables|Default|Setis%20Get%20Damage%20For%20Crash true))))

(event OnComponentBeginOverlap(PossesCollision)
  (params (OverlappedComponent :type Primitive%20Component%20Object%20Reference) (OtherActor :type Actor%20Object%20Reference) (OtherComp :type Primitive%20Component%20Object%20Reference) (OtherBodyIndex :type Integer) (bFromSweep :type Boolean) (SweepResult :type Hit%20Result%20Structure%20%28by%20ref%29))
  ;[0.1042 0.1042 0.1042] Show / Hide E Key
  (bind _asbpc_gezer (Utilities|Casting|CastToBPC_Gezer OtherActor))
  (Variables|Posses|SetBPC%20Gezer _asbpc_gezer)
  (CallFunction|Show/HideEKey true))

(event OnComponentEndOverlap(PossesCollision)
  (params (OverlappedComponent :type Primitive%20Component%20Object%20Reference) (OtherActor :type Actor%20Object%20Reference) (OtherComp :type Primitive%20Component%20Object%20Reference) (OtherBodyIndex :type Integer))
  ;[0.1042 0.1042 0.1042] Show / Hide E Key
  (Utilities|Casting|CastToBPC_Gezer OtherActor)
  (CallFunction|Show/HideEKey false))

(event Custom|Set%20Engine%20VFX%20Scale
  (params (Engine%20Scale :type Float%20%28double-precision%29))
  (bind _returnvalue (* Engine%20Scale 3.0))
  (bind _p_engineleft (Variables|Default|GetP_EngineLeft))
  (bind _p_engineleft_2 (Variables|Default|GetP_EngineLeft))
  (bind _p_engineright (Variables|Default|GetP_EngineRight))
  (bind _returnvalue_2 (Transformation|GetWorldScale _p_engineleft))
  (bind _returnvalue_3 (Transformation|GetWorldScale _p_engineleft_2))
  (bind _returnvalue_4 (Transformation|GetWorldScale _p_engineright))
  (bind _returnvalue_5 (Math|Float|Lerp (.z _returnvalue_2) _returnvalue 0.05))
  ;[0.1042 0.1042 0.1042] Set Space Engine VFX Scale
  (Transformation|SetWorldScale3D _p_engineleft_2 (Math|Vector|MakeVector (.x _returnvalue_3) (.y _returnvalue_3) _returnvalue_5))
  (Transformation|SetWorldScale3D _p_engineright (Math|Vector|MakeVector (.x _returnvalue_4) (.y _returnvalue_4) _returnvalue_5))
  (CallFunction|SetThrustSoundVolume Engine%20Scale))

(event Custom|Show%20/%20Hide%20E%20Key
  (params (Show :type Boolean))
  ;[0.1042 0.1042 0.1042] Show / Hide E Key
  (Default|Show/HideEKey (Variables|Default|GetWB%20E%20Key) Show "F"))

(event Custom|Update%20Health
  (params (HP%20Change%20Amount :type Float%20%28double-precision%29))
  ;[0.1042 0.1042 0.1042] HP System
  ;;[0.1042 0.1042 0.1042] Get Damage
  (Variables|HealthSystem|SetHealth (Math|Float|Clamp(Float) (+ (Variables|HealthSystem|GetHealth) HP%20Change%20Amount) 0.0 (Variables|HealthSystem|GetMax%20Health)))
  (CallFunction|SetHPPercent)
  (if (and (<= (Variables|HealthSystem|GetHealth) 0.0) (Variables|Default|Getis%20Alive))
    (CallFunction|Die)))

(event Custom|Die
  (bind _space_ship_mesh (Variables|Default|GetSpace%20Ship%20Mesh))
  ;[0.1042 0.1042 0.1042] HP System
  ;;[0.1042 0.1042 0.1042] Die Function
  (Variables|Default|Setis%20Alive false)
  (Input|DisableInput 0)
  (Physics|SetSimulatePhysics _space_ship_mesh true)
  (Physics|SetEnableGravity _space_ship_mesh true)
  (|DieEffect)
  (|RestartGame))

(event Custom|Set%20Thrust%20Sound%20Volume
  (params (A :type Float%20%28double-precision%29))
  (bind _space_engine_loop (Variables|Default|GetSpace_Engine_Loop))
  ;[0.1042 0.1042 0.1042] Set Engine Sound Amount
  (Audio|Components|Audio|SetVolumeMultiplier _space_engine_loop (Math|Float|Lerp (Variables|/Script/Engine.AudioComponent|GetVolumeMultiplier _space_engine_loop) (* A 0.2) 0.05) :!class /Script/Engine.AudioComponent))

(event Input|EnhancedActionEvents|EnhancedInputActionIA_Ship_UpDown
  (params (ActionValue :type Float%20%28double-precision%29) (ElapsedSeconds :type Float%20%28double-precision%29) (TriggeredSeconds :type Float%20%28double-precision%29) (InputAction :type Input%20Action%20Object%20Reference :default "/Game/-Yunus/Inputs/SpaceShip/IA_Ship_UpDown.IA_Ship_UpDown"))
  ;[0.4115 0.02786 0.02786] Set Thrust - Up / Down
  (:Triggered
    (Physics|AddForce (Variables|Default|GetSpace%20Ship%20Mesh) (* ActionValue (Transformation|GetActorUpVector) 5e+02) "None" true)))

(event Input|EnhancedActionEvents|EnhancedInputActionIA_Ship_Forward
  (params (ActionValue :type Float%20%28double-precision%29) (ElapsedSeconds :type Float%20%28double-precision%29) (TriggeredSeconds :type Float%20%28double-precision%29) (InputAction :type Input%20Action%20Object%20Reference :default "/Game/-Yunus/Inputs/SpaceShip/IA_Ship_Forward.IA_Ship_Forward"))
  ;[0.4115 0.02786 0.02786] Set Thrust - Forward
  (:Triggered
    (Physics|AddForce (Variables|Default|GetSpace%20Ship%20Mesh) (* (Transformation|GetActorForwardVector) ActionValue -1.0 2.5e+04) "None" true)
    ;[0.1042 0.1042 0.1042] Set Engine VFX
    (CallFunction|SetEngineVFXScale ActionValue))
  (:Completed
    (bind _vfx_scale (Timeline|Close%20Engine%20VFX PlayFromStart)
      (:Update
        (CallFunction|SetEngineVFXScale _vfx_scale)))))

(event Input|EnhancedActionEvents|EnhancedInputActionIA_Ship_Look
  (params (ActionValue :type Vector%202D%20Structure) (ElapsedSeconds :type Float%20%28double-precision%29) (TriggeredSeconds :type Float%20%28double-precision%29) (InputAction :type Input%20Action%20Object%20Reference :default "/Game/-Yunus/Inputs/SpaceShip/IA_Ship_Look.IA_Ship_Look"))
  ;[0.4115 0.02786 0.02786] Turn Pitch / Yaw
  (:Triggered
    (Class|PrimitiveComponent|AddTorqueinDegrees (Variables|Default|GetSpace%20Ship%20Mesh) (+ (* (.x ActionValue) (Transformation|GetActorUpVector) 2e+02) (* (.y ActionValue) (Transformation|GetActorRightVector) 2e+02 -1.0)) "None" true)))

(event Input|EnhancedActionEvents|EnhancedInputActionIA_Ship_Roll
  (params (ActionValue :type Float%20%28double-precision%29) (ElapsedSeconds :type Float%20%28double-precision%29) (TriggeredSeconds :type Float%20%28double-precision%29) (InputAction :type Input%20Action%20Object%20Reference :default "/Game/-Yunus/Inputs/SpaceShip/IA_Ship_Roll.IA_Ship_Roll"))
  ;[0.4115 0.02786 0.02786] Turn Roll
  (:Triggered
    (Class|PrimitiveComponent|AddTorqueinDegrees (Variables|Default|GetSpace%20Ship%20Mesh) (* ActionValue (Transformation|GetActorForwardVector) 8e+02) "None" true)))

(event Input|EnhancedActionEvents|EnhancedInputActionIA_Get_In-Out_Ship
  (params (ActionValue :type Boolean) (ElapsedSeconds :type Float%20%28double-precision%29) (TriggeredSeconds :type Float%20%28double-precision%29) (InputAction :type Input%20Action%20Object%20Reference :default "/Game/-Yunus/Inputs/Player/IA_Get_In-Out_Ship.IA_Get_In-Out_Ship"))
  (bind _returnvalue (Transformation|GetActorLocation))
  (bind _player_get_out_location (Variables|Default|GetPlayer%20Get%20Out%20Location))
  (bind _bpc_gezer (Variables|Posses|GetBPC%20Gezer))
  ;[0.4115 0.02786 0.02786] Get Out Space Ship
  (:Started
    ;;[0.1042 0.1042 0.1042] is Under Gound Check
    (bind _returnvalue_2 (Collision|LineTraceByChannel _returnvalue (+ _returnvalue (* -1e+02 (Transformation|GetActorUpVector))) "TraceTypeQuery1" false 0 "None"))
    (if _returnvalue_2
      (Default|Enable/DisablePlayer _bpc_gezer false (Transformation|GetWorldLocation _player_get_out_location) (.pitch (Transformation|GetWorldRotation _player_get_out_location)))
      (Pawn|Possess (Game|GetPlayerController 0) _bpc_gezer)
      (Default|WeaponShoworHide _bpc_gezer false))))

(event Input|EnhancedActionEvents|EnhancedInputActionIA_Ship_Right-Left
  (params (ActionValue :type Float%20%28double-precision%29) (ElapsedSeconds :type Float%20%28double-precision%29) (TriggeredSeconds :type Float%20%28double-precision%29) (InputAction :type Input%20Action%20Object%20Reference :default "/Game/-Yunus/Inputs/SpaceShip/IA_Ship_Right-Left.IA_Ship_Right-Left"))
  ;[0.4115 0.02786 0.02786] Set Thrust Right / Left
  (:Triggered
    (Physics|AddForce (Variables|Default|GetSpace%20Ship%20Mesh) (* ActionValue (Transformation|GetActorRightVector) 2.5e+03) "None" true)))

(event EventBeginPlay
  (CallFunction|SetIMC "/Game/-Yunus/Inputs/SpaceShip/IMC_SpaceShip.IMC_SpaceShip")
  (Variables|HealthSystem|SetHealth (Variables|HealthSystem|GetMax%20Health))
  (|SetWBEKey)
  ;[0.1042 0.1042 0.1042] When Player Start as Space Ship, set player isntance
  (Utilities|IsValid (Variables|Posses|GetBPC%20Gezer)
    (:Is%20Not%20Valid
      (bind _returnvalue (Actor|GetActorOfClass "/Game/MetaHumans/Taro/BP_Alper.BP_Alper_C"))
      (Variables|Posses|SetBPC%20Gezer _returnvalue))))

(event EventUpdateHPInterface
  (params (HP%20Change%20Amount :type Float%20%28double-precision%29))
  ;[0.1042 0.1042 0.1042] HP System
  (CallFunction|UpdateHealth HP%20Change%20Amount))

(event EventPossessed
  (params (NewController :type Controller%20Object%20Reference))
  ;[0.1042 0.1042 0.1042] Posses Work
  (Input|AddMappingContext (PlayerController|LocalPlayerSubsystems|GetEnhancedInputLocalPlayerSubsystem (Game|GetPlayerController 0)) "/Game/-Yunus/Inputs/SpaceShip/IMC_SpaceShip.IMC_SpaceShip" 0 "(bIgnoreAllPressedKeysUntilRelease=True,bForceImmediately=False)")
  (Physics|SetSimulatePhysics (Variables|Default|GetSpace%20Ship%20Mesh) true)
  (CallFunction|SetWidget)
  (|ChangeCurrentQuest 2)
  (|StartShieldregen))

(event EventUnpossessed
  (params (OldController :type Controller%20Object%20Reference))
  ;[0.1042 0.1042 0.1042] Posses Work
  (Input|RemoveMappingContext (PlayerController|LocalPlayerSubsystems|GetEnhancedInputLocalPlayerSubsystem (Game|GetPlayerController 0)) "/Game/-Yunus/Inputs/SpaceShip/IMC_SpaceShip.IMC_SpaceShip" "(bIgnoreAllPressedKeysUntilRelease=True,bForceImmediately=False)")
  (Physics|SetSimulatePhysics (Variables|Default|GetSpace%20Ship%20Mesh) false)
  (CallFunction|RemoveWidget))

(event Custom|Spawn%20Bullet
  (params (Bullet%20Muzzle :type Scene%20Component%20Object%20Reference))
  ;[0.1042 0.1042 0.1042] Spawn bullet
  (bind _returnvalue (Game|SpawnActorfromClass "/Game/-Yunus/Blueprints/Weapon/A_PlayerShip_LazerBullet.A_PlayerShip_LazerBullet_C" (Transformation|GetWorldTransform Bullet%20Muzzle) "Undefined" "MultiplyWithRoot" 0 0))
  (Default|SetStartValue _returnvalue (Variables|LazerMachine|GetBullet%20Speed) (Variables|LazerMachine|GetBullet%20Damage) (Variables|LazerMachine|GetBullet%20Life%20Time))
  (Audio|PlaySound2D "/Game/-Yunus/Sounds/Space_Ship/MS_Lazer_Gun.MS_Lazer_Gun" 0.4 1.0 0.0 0 0 false))

(event Input|EnhancedActionEvents|EnhancedInputActionIA_Ship_AttackMachineGun
  (params (ActionValue :type Boolean) (ElapsedSeconds :type Float%20%28double-precision%29) (TriggeredSeconds :type Float%20%28double-precision%29) (InputAction :type Input%20Action%20Object%20Reference :default "/Game/-Yunus/Inputs/SpaceShip/IA_Ship_AttackMachineGun.IA_Ship_AttackMachineGun"))
  ;[0.4115 0.02786 0.02786] Attack Lazer Machine Bullet
  (:Triggered
    (if (Variables|LazerMachine|GetCan%20Attack%20Lazer)
      (Variables|LazerMachine|SetCan%20Attack%20Lazer false)
      (CallFunction|SpawnBullet (Variables|Default|GetMachineGunLocation))
      (Utilities|FlowControl|Delay (Variables|LazerMachine|GetBullet%20Attack%20Speed))
      (Variables|LazerMachine|SetCan%20Attack%20Lazer true))))

(fn ConstructionScript)

(fn SetIMC
  (params (MappingContext :type Input%20Mapping%20Context%20Object%20Reference))
  (bind _asplayer_controller (Utilities|Casting|CastToPlayerController (Pawn|GetController)))
  (Utilities|IsValid (PlayerController|LocalPlayerSubsystems|GetEnhancedInputLocalPlayerSubsystem _asplayer_controller)
    (:Is%20Valid
      (Input|AddMappingContext (PlayerController|LocalPlayerSubsystems|GetEnhancedInputLocalPlayerSubsystem _asplayer_controller) MappingContext 0 "(bIgnoreAllPressedKeysUntilRelease=True,bForceImmediately=False)"))))

(fn SetWidget
  (bind _returnvalue (UserInterface|CreateWidget "/Game/-Yunus/UI/SpaceShip/WB_Kurt.WB_Kurt_C"))
  (bind _output_get (Variables|Posses|SetWB%20Kurt _returnvalue))
  (UserInterface|Viewport|AddtoViewport _output_get 0)
  (CallFunction|SetHPPercent))

(fn ShowSpeed
  (Development|PrintString (Utilities|String|ToString(Float) (Math|Vector|VectorLength (Transformation|GetComponentVelocity (Variables|Default|GetSpace%20Ship%20Mesh))))))

(fn RemoveWidget
  (Widget|RemovefromParent (Variables|Posses|GetWB%20Kurt)))

(fn SetHPPercent
  (Default|SetHPPercent (Variables|Posses|GetWB%20Kurt) (/ (Variables|HealthSystem|GetHealth) (Variables|HealthSystem|GetMax%20Health))))