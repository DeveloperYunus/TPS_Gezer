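; Enemy dummy character that tracks health, shows it through a widget-based health UI, and handles its own death.
; BeginPlay fills health and caches the WB_HealthUI widget, which custom events use to show damage numbers and update the health bar.
; Die clears the alive flag, plays a sound, hides the UI, ragdolls the mesh with reduced capsule collision, then drops mesh collision after a delay before destroying the actor.
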(event Custom|Die
  (bind _capsulecomponent (Variables|Collision|GetCapsuleComponent))
  ;[0.1042 0.1042 0.1042] Die
  (Variables|HealthSystem|Setis%20Alive false)
  (Audio|PlaySoundatLocation "/Game/-Yunus/Sounds/Enemy/Dead.Dead" "0, 0, 0" "0, 0, 0" 0.4 1.1 0.0 0 0 0 0)
  (Variables|/Script/UMG.Widget|SetVisibility (Variables|HealthSystem|GetHealth%20%20UI) "Hidden")
  (Physics|SetSimulatePhysics (Variables|Character|GetMesh) true)
  (Collision|SetCollisionResponsetoAllChannels _capsulecomponent "ECR_Ignore")
  (Collision|SetCollisionResponsetoChannel _capsulecomponent "ECC_WorldStatic" "ECR_Block")
  (Utilities|FlowControl|Delay 3.0)
  (Collision|SetCollisionResponsetoAllChannels (Variables|Character|GetMesh) "ECR_Ignore")
  (Utilities|FlowControl|Delay 1.0)
  (Actor|DestroyActor))

(event Custom|Show%20Taken%20Damage
  (params (Damage%20Amount :type Float%20%28double-precision%29))
  ;[0.1042 0.1042 0.1042] Show Damage
  (Default|ShowDamage (Variables|HealthSystem|GetHealth%20%20UI) (Utilities|Text|ToText(Float) Damage%20Amount "HalfToEven")))

(event Custom|Update%20Health%20Bar
  ;[0.1042 0.1042 0.1042] Update HP Bar
  (Default|UpdateHealthBar (Variables|HealthSystem|GetHealth%20%20UI) (/ (Variables|HealthSystem|GetHealth) (Variables|HealthSystem|GetMax%20Health))))

(event EventBeginPlay
  (Variables|HealthSystem|SetHealth (Variables|HealthSystem|GetMax%20Health))
  ;[0.1042 0.1042 0.1042] Cast Damage UI
  (bind _aswb_health_ui (Utilities|Casting|CastToWB_HealthUI (UserInterface|GetWidget (Variables|Default|GetHealth%20UI))))
  (Variables|HealthSystem|SetHealth%20%20UI _aswb_health_ui))

(fn ConstructionScript)