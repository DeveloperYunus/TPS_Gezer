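; Sword-wielding enemy character that draws, sheathes and slashes with a katana, and exposes a patrol route and movement speed setting.
; Montages drive the actions, reattaching the sword between hand and sheath sockets and firing callbacks when sheathing or attacks end.
; A looping timer sphere-traces along the blade with debug drawing, damaging BPC_Gezer once per trace window with blood and sound effects.
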(event Custom|Attack%20Sword
  ;[0.1042 0.1042 0.1042] Attack Sword
  (if (Variables|Default|Getis%20Wielding%20Sword)
    (Animation|Montage|PlayMontage (Variables|Character|GetMesh) "/Game/-Yunus/Animations/Katana/Katana_Slash_Montage.Katana_Slash_Montage"
      (:OnCompleted
        _)
      (:OnInterrupted
        _))
    (Default|CallOnAttackEnd)))

(event Custom|Wield%20Sword
  ;[0.1042 0.1042 0.1042] Wield Sword
  (Animation|Montage|PlayMontage (Variables|Character|GetMesh) "/Game/-Yunus/Animations/Katana/KatanaOut_Montage.KatanaOut_Montage"
    (:then
      (Utilities|FlowControl|Delay 0.2)
      (Transformation|AttachComponentToComponent (Variables|Default|GetSword%20Actor) (Variables|Character|GetMesh) "Katana_Hand_Socket" "SnapToTarget" "SnapToTarget" "SnapToTarget" true)
      (Variables|Default|Setis%20Wielding%20Sword true))))

(event Custom|Unwield%20Sword
  ;[0.1042 0.1042 0.1042] Unwield Sword
  (bind _notifyname (Animation|Montage|PlayMontage (Variables|Character|GetMesh) "/Game/-Yunus/Animations/Katana/KatanaIn_Montage.KatanaIn_Montage")
    (:OnCompleted
      (Default|CallOnUnweildSword))
    (:OnNotifyBegin
      (switch name _notifyname
        (:Sword%20In
          (Transformation|AttachComponentToComponent (Variables|Default|GetSword%20Actor) (Variables|Default|GetSword) "Katana_Default_Socket" "SnapToTarget" "SnapToTarget" "SnapToTarget" true)
          (Variables|Default|Setis%20Wielding%20Sword false))))))

(event Custom|Sword%20Trace%20Start
  ;[0.1042 0.1042 0.1042] Sword Trace System
  (bind _outhit (Collision|SphereTraceByChannel (Transformation|GetWorldLocation (Variables|Default|GetTraceStart)) (Transformation|GetWorldLocation (Variables|Default|GetTraceEnd)) 1e+01 "TraceTypeQuery1" false 0 "ForDuration" true "(R=1.000000,G=0.000000,B=0.000000,A=1.000000)" "(R=0.000000,G=1.000000,B=0.000000,A=1.000000)" 0.1))
  (bind _asbpc_gezer (Utilities|Casting|CastToBPC_Gezer (.HitActor (Collision|BreakHitResult _outhit))))
  ;[0.1042 0.1042 0.1042] Sword Cut Effects
  (if (Variables|Default|GetCan%20Give%20Damage)
    (Effects|SpawnEmitteratLocation "/Game/Realistic_Starter_VFX/Particles/Blood/P_Blood_Splat_Cone.P_Blood_Splat_Cone" (.ImpactPoint (Collision|BreakHitResult _outhit)) (Math|Rotator|MakeRotfromZ (.Normal (Collision|BreakHitResult _outhit))) "0.700000,0.700000,0.500000")
    (Audio|SpawnSoundatLocation "/Game/-Yunus/Sounds/Weapons/Katana/Sword_Slash.Sword_Slash" (.ImpactPoint (Collision|BreakHitResult _outhit)) "0, 0, 0" 0.2 1.5 0.0 0 0)
    (Default|UpdateHealth _asbpc_gezer (Variables|Default|GetSword%20Damage))
    (Variables|Default|SetCan%20Give%20Damage false)))

(event Custom|Start%20Sword%20Trace
  ;[0.1042 0.1042 0.1042] Sword Trace System
  (bind _returnvalue (Utilities|Time|SetTimerbyEvent (delegate Custom|Sword%20Trace%20Start) 0.02 true))
  (Variables|Default|SetSword%20Trace%20Timer _returnvalue)
  (Variables|Default|SetCan%20Give%20Damage true))

(event Custom|Sword%20Trace%20End
  ;[0.1042 0.1042 0.1042] Sword Trace System
  (Utilities|Time|ClearandInvalidateTimerbyHandle (Variables|Default|GetSword%20Trace%20Timer)))

(event EventBeginPlay
  ;[0.1042 0.1042 0.1042] Begin Settings
  (|CallParentFunction))

(fn ConstructionScript
  (|CallParentFunction))

(fn GetPatrolRoute
  (return (Variables|Default|GetPatrolRoute)))

(fn SetMovementSpeed
  (params (Speed :type E_MovementSpeed%20Enum :default "NewEnumerator0"))
  (Variables|/Script/Engine.CharacterMovementComponent|SetMaxWalkSpeed (Variables|Character|GetCharacterMovement) (Utilities|Select :Index Speed :NewEnumerator0 0.0 :NewEnumerator1 2e+02 :NewEnumerator2 5.8e+02 :NewEnumerator3 7e+02))
  (return 0.0))