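; BP_ControlPanel is an interactable control panel that the player destroys to win the level.
; While active, its box overlap toggles an E-key prompt widget and binds or unbinds destruction to BPC_Gezer's interact event.
; Interacting deactivates the panel, spawns a delayed smoke explosion, flickers the PanelUI actor off through chained timed visibility toggles, then calls WinGame on GM_SpaceShip after a pause.
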(event OnComponentBeginOverlap(Box)
  (params (OverlappedComponent :type Primitive%20Component%20Object%20Reference) (OtherActor :type Actor%20Object%20Reference) (OtherComp :type Primitive%20Component%20Object%20Reference) (OtherBodyIndex :type Integer) (bFromSweep :type Boolean) (SweepResult :type Hit%20Result%20Structure%20%28by%20ref%29))
  ;[0.1042 0.1042 0.1042] Overlap Begin / End
  (if (Variables|Default|Getis%20Panel%20Active)
    (bind _asbpc_gezer (Utilities|Casting|CastToBPC_Gezer OtherActor))
    (Variables|Default|SetBPC%20Gezer _asbpc_gezer)
    (CallFunction|Show/HideEKey true)
    (EventDispatchers|BindEventtoInteractObject (Variables|Default|GetBPC%20Gezer) (delegate Custom|Destroy%20Panel%20UI%20Bind))))

(event OnComponentEndOverlap(Box)
  (params (OverlappedComponent :type Primitive%20Component%20Object%20Reference) (OtherActor :type Actor%20Object%20Reference) (OtherComp :type Primitive%20Component%20Object%20Reference) (OtherBodyIndex :type Integer))
  ;[0.1042 0.1042 0.1042] Overlap Begin / End
  (if (Variables|Default|Getis%20Panel%20Active)
    (Utilities|Casting|CastToBPC_Gezer OtherActor)
    (CallFunction|Show/HideEKey false)
    (EventDispatchers|UnbindEventfromInteractObject (Variables|Default|GetBPC%20Gezer) (delegate Custom|Destroy%20Panel%20UI%20Bind))))

(event Custom|Explosion%20Effect
  (Effects|SpawnEmitterAttached "/Game/Realistic_Starter_VFX/Particles/Explosion/P_Explosion_Smoke.P_Explosion_Smoke" (Variables|Default|GetExplosion%20Point) "None" "0, 0, 0" "0, 0, 0" "0.250000,0.250000,0.250000"))

(event Custom|Show%20/%20Hide%20E%20Key
  (params (Show :type Boolean))
  (Default|Show/HideEKey (Variables|Default|GetWB%20E%20Key) Show))

(event Custom|Destroy%20Panel%20UI
  (Variables|Default|Setis%20Panel%20Active false)
  (CallFunction|Show/HideEKey false)
  (Utilities|FlowControl|Delay 2.0)
  (CallFunction|ExplosionEffect)
  (Utilities|FlowControl|Delay 1.0)
  (|Show/HidePanelUI 0.2 true
    (:Completed
      (|Show/HidePanelUI_2 0.05 false
        (:Completed
          (|Show/HidePanelUI_2_2 0.3 true
            (:Completed
              (|WinGame))))))))

(event Custom|Destroy%20Panel%20UI%20Bind
  ;[0.1042 0.1042 0.1042] Overlap Begin / End
  (CallFunction|DestroyPanelUI))

(event EventBeginPlay
  (bind _aswb_e_key (Utilities|Casting|CastToWB_E_Key (UserInterface|GetWidget (Variables|Default|GetWidget))))
  (Variables|Default|SetWB%20E%20Key _aswb_e_key))

(fn ConstructionScript)