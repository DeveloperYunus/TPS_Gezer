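; BP_DesertCaveIn is a desert level trigger with a gate, apparently marking a cave entrance that the spaceship reaches against a closing timer.
; The first overlap of its Box by BPP_SpaceShip tells the cached GM_SpaceShip game mode to stop the gate-closing timing.
; A separate CloseGate event, not called within this Blueprint, drops the referenced Gate actor instantly by a fixed local Z offset.
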(event OnComponentBeginOverlap(Box)
  (params (OverlappedComponent :type Primitive%20Component%20Object%20Reference) (OtherActor :type Actor%20Object%20Reference) (OtherComp :type Primitive%20Component%20Object%20Reference) (OtherBodyIndex :type Integer) (bFromSweep :type Boolean) (SweepResult :type Hit%20Result%20Structure%20%28by%20ref%29))
  (if (Variables|Default|Getis%20First%20Enter)
    (Utilities|Casting|CastToBPP_SpaceShip OtherActor)
    (Default|StopClosingGateTiming (Variables|Default|GetGM%20Space%20Ship))
    (Variables|Default|Setis%20First%20Enter false)))

(event Custom|Close%20Gate
  (Transformation|AddActorLocalOffset (Variables|Default|GetGate) "0.000000,0.000000,-350.000000" false false))

(event EventBeginPlay
  (bind _asgm_space_ship (Utilities|Casting|CastToGM_SpaceShip (Game|GetGameMode)))
  (Variables|Default|SetGM%20Space%20Ship _asgm_space_ship))

(fn ConstructionScript)