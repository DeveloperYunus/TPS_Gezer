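; BP_Door is an interactive door that the BPC_Gezer character can open and close.
; Entering its box trigger shows an E-key widget and binds the door toggle to the character's interact event; leaving hides and unbinds it.
; Each interaction alternates through a FlipFlop between open and close timelines that rotate the mesh yaw, scaled to 90 degrees.
; A usability flag blocks input until the current swing finishes.
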(event OnComponentBeginOverlap(Box)
  (params (OverlappedComponent :type Primitive%20Component%20Object%20Reference) (OtherActor :type Actor%20Object%20Reference) (OtherComp :type Primitive%20Component%20Object%20Reference) (OtherBodyIndex :type Integer) (bFromSweep :type Boolean) (SweepResult :type Hit%20Result%20Structure%20%28by%20ref%29))
  ;[0.1042 0.1042 0.1042] Player Door Event (In = Bind / Out = Unbind)
  (bind _asbpc_gezer (Utilities|Casting|CastToBPC_Gezer OtherActor))
  (Variables|Default|SetBPC%20Gezer _asbpc_gezer)
  (CallFunction|Show/HideEKey true)
  (EventDispatchers|BindEventtoInteractObject (Variables|Default|GetBPC%20Gezer) (delegate Custom|Open%20Close%20Door%20Bind)))

(event OnComponentEndOverlap(Box)
  (params (OverlappedComponent :type Primitive%20Component%20Object%20Reference) (OtherActor :type Actor%20Object%20Reference) (OtherComp :type Primitive%20Component%20Object%20Reference) (OtherBodyIndex :type Integer))
  ;[0.1042 0.1042 0.1042] Player Door Event (In = Bind / Out = Unbind)
  (Utilities|Casting|CastToBPC_Gezer OtherActor)
  (CallFunction|Show/HideEKey false)
  (EventDispatchers|UnbindEventfromInteractObject (Variables|Default|GetBPC%20Gezer) (delegate Custom|Open%20Close%20Door%20Bind)))

(event Custom|Open%20Close%20Door%20Bind
  ;[0.1042 0.1042 0.1042] Player Door Event (In = Bind / Out = Unbind)
  (CallFunction|OpenCloseDoor))

(event Custom|Show%20/%20Hide%20E%20Key
  (params (Show :type Boolean))
  (Default|Show/HideEKey (Variables|Default|GetWB%20E%20Key) Show))

(event Custom|Open%20Close%20Door
  ;[0.4115 0.02786 0.02786] Door Open Close Event
  (if (Variables|Default|Getcan%20Door%20Usable)
    (Variables|Default|Setcan%20Door%20Usable false)
    (Utilities|FlowControl|FlipFlop
      (:A
        (bind _open_door (Timeline|Open%20Door PlayFromStart)
          (:Update
            (Transformation|SetRelativeRotation (Variables|Default|GetDoor%20Mesh) (Math|Rotator|MakeRotator 0.0 0.0 (* _open_door 9e+01)) false false))
          (:Finished
            (Variables|Default|Setcan%20Door%20Usable true :!label _label))))
      (:B
        (bind _close_door (Timeline|Timeline PlayFromStart)
          (:Update
            (Transformation|SetRelativeRotation (Variables|Default|GetDoor%20Mesh) (Math|Rotator|MakeRotator 0.0 0.0 (* _close_door 9e+01)) false false))
          (:Finished
            (goto _label)))))))

(event EventBeginPlay
  (bind _aswb_e_key (Utilities|Casting|CastToWB_E_Key (UserInterface|GetWidget (Variables|Default|GetWidget))))
  (Variables|Default|SetWB%20E%20Key _aswb_e_key))

(fn ConstructionScript)