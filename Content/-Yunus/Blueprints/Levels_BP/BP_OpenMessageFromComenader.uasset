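; Interactable trigger that lets the player open and close the commander's message in the player UI.
; Overlapping its box shows an E key widget and binds the toggle to BPC_Gezer's interact event; leaving hides it, unbinds, and closes any open message.
; Opening the message also advances the current quest through GM_CoreScene.
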(event OnComponentBeginOverlap(Box)
  (params (OverlappedComponent :type Primitive%20Component%20Object%20Reference) (OtherActor :type Actor%20Object%20Reference) (OtherComp :type Primitive%20Component%20Object%20Reference) (OtherBodyIndex :type Integer) (bFromSweep :type Boolean) (SweepResult :type Hit%20Result%20Structure%20%28by%20ref%29))
  ;[0.1042 0.1042 0.1042] Player Door Event (In = Bind / Out = Unbind)
  (bind _asbpc_gezer (Utilities|Casting|CastToBPC_Gezer OtherActor))
  (Variables|Default|SetBPC%20Gezer _asbpc_gezer)
  (CallFunction|Show/HideEKey true)
  (EventDispatchers|BindEventtoInteractObject (Variables|Default|GetBPC%20Gezer) (delegate Custom|E%20Key%20Function%20Event)))

(event OnComponentEndOverlap(Box)
  (params (OverlappedComponent :type Primitive%20Component%20Object%20Reference) (OtherActor :type Actor%20Object%20Reference) (OtherComp :type Primitive%20Component%20Object%20Reference) (OtherBodyIndex :type Integer))
  ;[0.1042 0.1042 0.1042] Player Door Event (In = Bind / Out = Unbind)
  (Utilities|Casting|CastToBPC_Gezer OtherActor)
  (CallFunction|Show/HideEKey false)
  (EventDispatchers|UnbindEventfromInteractObject (Variables|Default|GetBPC%20Gezer) (delegate Custom|E%20Key%20Function%20Event))
  (if (Variables|Default|Getis%20Message%20Panel%20Open)
    ;[0.1042 0.1042 0.1042] Comanders Message On / Off
    (Default|On/OffCOmanderText (Variables|/Game/-Yunus/Blueprints/BPC_Gezer.BPC_Gezer_C|GetPlayer%20UI (Variables|Default|GetBPC%20Gezer)) "Reverse")
    (Variables|Default|Setis%20Message%20Panel%20Open false)))

(event Custom|E%20Key%20Function%20Event
  ;[0.1042 0.1042 0.1042] Player Door Event (In = Bind / Out = Unbind)
  (CallFunction|EKeyFunction false))

(event Custom|Show%20/%20Hide%20E%20Key
  (params (Show :type Boolean))
  (Default|Show/HideEKey (Variables|Default|GetWB%20E%20Key) Show))

(event Custom|E%20Key%20Function
  (params (Out%20Close :type Boolean))
  (bind _bpc_gezer (Variables|Default|GetBPC%20Gezer))
  (bind _player_ui (Variables|/Game/-Yunus/Blueprints/BPC_Gezer.BPC_Gezer_C|GetPlayer%20UI _bpc_gezer))
  ;[0.1042 0.1042 0.1042] Comanders Message On / Off
  (if (Variables|Default|Getis%20Message%20Panel%20Open)
    (Default|On/OffCOmanderText _player_ui "Reverse")
    (Variables|Default|Setis%20Message%20Panel%20Open false)
    (else
      (Default|On/OffCOmanderText _player_ui "Forward")
      (Variables|Default|Setis%20Message%20Panel%20Open true)
      (|ChangeCurrentQuest 1))))

(event EventBeginPlay
  (bind _aswb_e_key (Utilities|Casting|CastToWB_E_Key (UserInterface|GetWidget (Variables|Default|GetWidget))))
  (Variables|Default|SetWB%20E%20Key _aswb_e_key))

(fn ConstructionScript)