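; GM_CoreScene, apparently a game mode, drives the screen transitions of the core scene and the travel to the DesertCity level.
; On BeginPlay it creates the WB_LevelTransitionUI widget, adds it to the viewport and plays its opening background animation forward.
; ChangeLevel starts the widget's warp effect, ends it after a timed delay, then opens DesertCity following a second short delay.
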(event Custom|Change%20Level
  (bind _level_transition_ui (Variables|Default|GetLevel%20Transition%20UI))
  (Default|PlayWarpEffect _level_transition_ui)
  (Utilities|FlowControl|Delay 4.0)
  (Default|EndWarpEffect _level_transition_ui)
  (Utilities|FlowControl|Delay 1.0)
  (Game|OpenLevel(byObjectReference) "/Game/-Yunus/Maps/DesertCity.DesertCity"))

(event Custom|Play%20Opening%20BG%20Anim
  (params (PlayMode :type EUMGSequencePlayMode%20Enum :default "Forward"))
  (Default|PlayOpeningBGAnim (Variables|Default|GetLevel%20Transition%20UI) PlayMode))

(event EventBeginPlay
  (bind _returnvalue (UserInterface|CreateWidget "/Game/-Yunus/UI/Level/WB_LevelTransitionUI.WB_LevelTransitionUI_C"))
  (bind _output_get (Variables|Default|SetLevel%20Transition%20UI _returnvalue))
  (UserInterface|Viewport|AddtoViewport _output_get 0)
  (CallFunction|PlayOpeningBGAnim "Forward"))

(fn ConstructionScript)