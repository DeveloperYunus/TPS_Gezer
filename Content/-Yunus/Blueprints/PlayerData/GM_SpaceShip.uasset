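; Game mode for the spaceship level that runs a timed escape before a gate closes and handles winning.
; After a short delay, a half-second Delay loop counts down and updates the LevelTransitionUI progress display until stopped.
; On timeout, the CheckTimeIsOver macro closes the BP_DesertCaveIn gate and reloads the current level.
; WinGame plays a reversed transition, disables input, destroys BPC_EnemySword actors and opens OurHome from inside that loop.
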(event Custom|Start%20Timing%20For%20Closing%20Gate
  (Default|SetRemainingTimeBeforeCloseGate (Variables|Default|GetLevel%20Transition%20UI) (/ (Variables|Default|GetDoor%20Close%20Second%20Timer) (Variables|Default|GetDoor%20Close%20Second)) :!label _label)
  (if (Variables|Default|Getis%20Timer%20Active)
    (Utilities|FlowControl|Delay 0.5)
    (Variables|Default|SetDoor%20Close%20Second%20Timer (- (Variables|Default|GetDoor%20Close%20Second%20Timer) 0.5))
    (|CheckTimeIsOver
      (:OutputPin
        (goto _label)))))

(event Custom|Stop%20Closing%20Gate%20Timing
  (Variables|Default|Setis%20Timer%20Active false)
  (Default|HideGateCloseTime (Variables|Default|GetLevel%20Transition%20UI)))

(event Custom|Win%20Game
  (Default|PlayOpeningBGAnim (Variables|Default|GetLevel%20Transition%20UI) "Reverse")
  (Utilities|FlowControl|Delay 1.0)
  (Input|DisableInput (Game|GetPlayerCharacter 0) 0)
  (bind _outactors (Actor|GetAllActorsOfClass "/Game/-Yunus/Blueprints/Enemy/BPC_EnemySword.BPC_EnemySword_C"))
  (for _array_element _outactors
    (Actor|DestroyActor _array_element)
    (Utilities|FlowControl|Delay 2.0)
    (Game|OpenLevel(byObjectReference) "/Game/-Yunus/Maps/OurHome.OurHome")))

(event EventBeginPlay
  (|CallParentFunction)
  (Default|ShowGateCloseTime (Variables|Default|GetLevel%20Transition%20UI))
  (Default|SetRemainingTimeBeforeCloseGate (Variables|Default|GetLevel%20Transition%20UI) 1.0)
  (Utilities|FlowControl|Delay 3.0)
  (CallFunction|StartTimingforClosingGate))

(fn ConstructionScript
  (|CallParentFunction))