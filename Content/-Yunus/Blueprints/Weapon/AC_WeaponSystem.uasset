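; Weapon system component for the BPC_Gezer player character that switches between unarmed, pistol and rifle states and provides firing helpers.
; WeaponState sets the character's animation state, returns both weapon child actors to holster sockets, then snaps the chosen one to a hand socket, using a separate rifle socket while sprinting.
; Separate functions provide a camera-forward line trace, fire sound and attached muzzle effect.
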(event Custom|Weapon%20State
  (params (Animation%20State :type Animation_State%20Enum :default "NewEnumerator0"))
  (bind _output_get (Variables|/Game/-Yunus/Blueprints/BPC_Gezer.BPC_Gezer_C|SetE_AnimationState (Variables|Default|GetBPC%20Gezer) Animation%20State))
  (bind _output_get_2 (Variables|Default|SetAnimation%20State _output_get))
  (switch Utilities|FlowControl|Switch|SwitchonAnimation_State _output_get_2
    (:NewEnumerator0
      (CallFunction|UnequipAll))
    (:NewEnumerator1
      (CallFunction|PistolEquip))
    (:NewEnumerator2
      (CallFunction|RifleEquip))))

(event EventBeginPlay
  (bind _asbpc_gezer (Utilities|Casting|CastToBPC_Gezer (Game|GetPlayerCharacter 0)))
  (Variables|Default|SetBPC%20Gezer _asbpc_gezer))

(fn RifleEquip
  (bind _bpc_gezer (Variables|Default|GetBPC%20Gezer))
  (bind _bpc_gezer_2 (Variables|Default|GetBPC%20Gezer))
  (CallFunction|UnequipAll)
  (ChildActorComponent|SetChildActorClass (Variables|/Game/-Yunus/Blueprints/BPC_Gezer.BPC_Gezer_C|GetRifleActor (Variables|Default|GetBPC%20Gezer)) "/Game/-Yunus/Blueprints/Weapon/BP_Rifle.BP_Rifle_C")
  (if (Variables|/Game/-Yunus/Blueprints/BPC_Gezer.BPC_Gezer_C|Getis%20Sprinting (Variables|Default|GetBPC%20Gezer))
    (Transformation|AttachComponentToComponent (Variables|/Game/-Yunus/Blueprints/BPC_Gezer.BPC_Gezer_C|GetRifleActor _bpc_gezer_2) (Variables|/Script/Engine.Character|GetMesh _bpc_gezer_2) "Rifle_Hand_Jog_Socket" "SnapToTarget" "SnapToTarget" "SnapToTarget" true)
    (else
      (Transformation|AttachComponentToComponent (Variables|/Game/-Yunus/Blueprints/BPC_Gezer.BPC_Gezer_C|GetRifleActor _bpc_gezer) (Variables|/Script/Engine.Character|GetMesh _bpc_gezer) "Rifle_Hand_Socket" "SnapToTarget" "SnapToTarget" "SnapToTarget" true))))

(fn PistolEquip
  (bind _bpc_gezer (Variables|Default|GetBPC%20Gezer))
  (CallFunction|UnequipAll)
  (ChildActorComponent|SetChildActorClass (Variables|/Game/-Yunus/Blueprints/BPC_Gezer.BPC_Gezer_C|GetPistolActor (Variables|Default|GetBPC%20Gezer)) "/Game/-Yunus/Blueprints/Weapon/BP_Pistol.BP_Pistol_C")
  (Transformation|AttachComponentToComponent (Variables|/Game/-Yunus/Blueprints/BPC_Gezer.BPC_Gezer_C|GetPistolActor _bpc_gezer) (Variables|/Script/Engine.Character|GetMesh _bpc_gezer) "Pistol_Hand_Socket" "SnapToTarget" "SnapToTarget" "SnapToTarget" true))

(fn UnequipAll
  (bind _bpc_gezer (Variables|Default|GetBPC%20Gezer))
  (bind _bpc_gezer_2 (Variables|Default|GetBPC%20Gezer))
  ;[0.1042 0.1042 0.1042] Rifle Unequip
  (ChildActorComponent|SetChildActorClass (Variables|/Game/-Yunus/Blueprints/BPC_Gezer.BPC_Gezer_C|GetRifleActor (Variables|Default|GetBPC%20Gezer)) "/Game/-Yunus/Blueprints/Weapon/BP_Rifle.BP_Rifle_C")
  (Transformation|AttachComponentToComponent (Variables|/Game/-Yunus/Blueprints/BPC_Gezer.BPC_Gezer_C|GetRifleActor _bpc_gezer_2) (Variables|/Game/-Yunus/Blueprints/BPC_Gezer.BPC_Gezer_C|GetRifle _bpc_gezer_2) "Rifle_Host_Socket" "SnapToTarget" "SnapToTarget" "SnapToTarget" true)
  ;[0.1042 0.1042 0.1042] Pistol Unequip
  (ChildActorComponent|SetChildActorClass (Variables|/Game/-Yunus/Blueprints/BPC_Gezer.BPC_Gezer_C|GetPistolActor (Variables|Default|GetBPC%20Gezer)) "/Game/-Yunus/Blueprints/Weapon/BP_Pistol.BP_Pistol_C")
  (Transformation|AttachComponentToComponent (Variables|/Game/-Yunus/Blueprints/BPC_Gezer.BPC_Gezer_C|GetPistolActor _bpc_gezer) (Variables|/Game/-Yunus/Blueprints/BPC_Gezer.BPC_Gezer_C|GetPistol _bpc_gezer) "Pistol_Host_Socket" "SnapToTarget" "SnapToTarget" "SnapToTarget" true))

(fn LineTrace
  (params (Animation%20State :type Animation_State%20Enum :default "NewEnumerator0") (Range :type Float%20%28single-precision%29))
  (bind _returnvalue (Game|GetPlayerCameraManager 0))
  (bind _returnvalue_2 (Camera|GetCameraLocation _returnvalue))
  (if (not (Utilities|Enum|Equal(Enum) Animation%20State (Variables|Default|GetAnimation%20State)))
    (bind (_outhit _returnvalue_3) (Collision|LineTraceByChannel _returnvalue_2 (+ _returnvalue_2 (* (Transformation|GetActorForwardVector _returnvalue) Range)) "TraceTypeQuery1" false 0 "None"))
    (if _returnvalue_3
      (return (.Location (Collision|BreakHitResult _outhit)) (.Normal (Collision|BreakHitResult _outhit)) (.HitActor (Collision|BreakHitResult _outhit)))
      (else
        (return "0, 0, 0" "0, 0, 0" 0)))))

(fn FireFX
  (params (Sound :type Sound%20Base%20Object%20Reference) (Location :type Vector) (VolumeMultiplier :type Float%20%28single-precision%29))
  (Audio|SpawnSoundatLocation Sound Location "0, 0, 0" VolumeMultiplier 1.0 0.0 0 0))

(fn MuzzleVFX
  (params (EmitterTemplate :type Particle%20System%20Object%20Reference) (AttachToComponent :type Scene%20Component%20Object%20Reference) (Scale :type Vector))
  (Effects|SpawnEmitterAttached EmitterTemplate AttachToComponent "None" "0, 0, 0" "0.000000,0.000000,80.000000" Scale))