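; Rifle weapon actor that implements hitscan firing, delegating most of the work to a WeaponSystem.
; Fire runs the WeaponSystem line trace over the rifle's range and passes the resulting location to FireFX along with the rifle shot sound.
; It then spawns a scaled-down particle effect on the Muzzle component and plays the fire animation on the weapon mesh.
; Reload is an empty event.
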(event EventBeginPlay
  (|CallParentFunction) ; This node is disabled and will not be called.\nDrag off pins to build functionality.
)

(event Collision|EventActorBeginOverlap
  (params (OtherActor :type Actor%20Object%20Reference))
  (|CallParentFunction OtherActor) ; This node is disabled and will not be called.\nDrag off pins to build functionality.
)

(event EventTick
  (params (DeltaSeconds :type Float%20%28single-precision%29))
  (|CallParentFunction DeltaSeconds) ; This node is disabled and will not be called.\nDrag off pins to build functionality.
)

(event EventReload)

(event EventFire
  (bind _weaponsystem (Variables|Default|GetWeaponSystem))
  (bind _location (Default|LineTrace _weaponsystem "NewEnumerator2" (Variables|Default|GetRifle%20Range)))
  (Default|FireFX _weaponsystem "/Game/-Yunus/Sounds/Weapons/Rifle/Weapons_Rifle_Noise-Exterior-Close_01.Weapons_Rifle_Noise-Exterior-Close_01" _location (Variables|Default|GetVolume%20Multiplier))
  (Default|MuzzleVFX _weaponsystem "/Game/Realistic_Starter_VFX_Pack_Vol2/Particles/Hit/P_Ceramic.P_Ceramic" (Variables|Default|GetMuzzle) "0.500000,0.500000,0.500000")
  (Components|Animation|PlayAnimation (Variables|Default|GetWeaponMesh) "/Game/-Yunus/Geometry/Weapon/Rifle/Animations/Weap_Rifle_Fire.Weap_Rifle_Fire" false))

(fn ConstructionScript
  (|CallParentFunction))